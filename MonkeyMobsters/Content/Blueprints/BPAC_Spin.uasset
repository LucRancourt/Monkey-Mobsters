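; BPAC_Spin is an actor component that makes its owning actor spin in yaw and bob up and down.
; BeginPlay caches the owner's starting height, then each Tick runs Spin and Float.
; Float ping-pongs a linear Lerp alpha to offset Z around that height, scaled by delta time, while Spin adds a fixed yaw per frame.
; The TryLoopLerp function is an empty stub.
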(event Custom|Spin
  ;[0.15 0.15 0.15 0.5] Spin
  (Transformation|AddActorLocalRotation (Components|GetOwner) (Math|Rotator|MakeRotator 0.0 0.0 (Variables|Default|GetSpinSpeed)) false false))

(event Custom|Float
  (bind _returnvalue (Components|GetOwner))
  (bind _returnvalue_2 (Utilities|Time|GetWorldDeltaSeconds))
  (bind _floatspeed (Variables|Default|GetFloatSpeed))
  (bind _returnvalue_3 (Transformation|GetActorLocation _returnvalue))
  (bind _returnvalue_4 (* _floatspeed _returnvalue_2))
  ;[0.15 0.15 0.15 0.5] Float
  (if (Variables|Default|GetbIsAdding)
    (Variables|Default|SetFloatAlpha (+ _returnvalue_4 (Variables|Default|GetFloatAlpha)))
    (else
      (Variables|Default|SetFloatAlpha (- (Variables|Default|GetFloatAlpha) _returnvalue_4))))
  (Transformation|SetActorLocation _returnvalue (Math|Vector|MakeVector (.x _returnvalue_3) (.y _returnvalue_3) (+ (* (Variables|Default|GetFloatHeight) (Math|Float|Lerp -1.0 1.0 (Variables|Default|GetFloatAlpha))) (Variables|Default|GetDefaultHeight))) false false)
  (if (or (>= (Variables|Default|GetFloatAlpha) 1.0) (<= (Variables|Default|GetFloatAlpha) 0.0))
    (Variables|Default|SetbIsAdding (not (Variables|Default|GetbIsAdding)))))

(event EventTick
  (params (DeltaSeconds :type Float%20%28single-precision%29))
  ;[0.15 0.15 0.15 0.5] Tick
  (Utilities|FlowControl|Sequence
    (:then_0
      (CallFunction|Spin))
    (:then_1
      (CallFunction|Float))))

(event EventBeginPlay
  ;[0.15 0.15 0.15 0.5] BeginPlay
  (Variables|Default|SetDefaultHeight (.z (Transformation|GetActorLocation (Components|GetOwner)))))

(fn TryLoopLerp)